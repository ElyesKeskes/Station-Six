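; BP_Devourer is an enemy character that stalks the player, freezing when seen and chasing when unseen.
; Each tick, a sphere trace finds the nearby player; recent mesh rendering plus a clear trace to the camera halts movement and animation.
; Without a detected player it attempts random navmesh wandering with breathing audio.
; A tazed flag read from its anim instance overrides this, stopping movement and playing a one-shot sound.
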(event EventTick
  (params (DeltaSeconds :type Float%20%28single-precision%29))
  (bind _returnvalue (Transformation|GetActorLocation))
  (bind _self self)
  (bind _devoureraudio (Variables|Default|GetDevourerAudio))
  (bind _devoureraudio_2 (Variables|Default|GetDevourerAudio))
  (bind _randomlocation (AI|Navigation|GetRandomReachablePointinRadius _returnvalue 1.5e+03 0 0))
  (bind _returnvalue_2 (Transformation|GetActorLocation _self))
  (bind _asdevourer_anim (Utilities|Casting|CastToDevourerAnim (Components|SkeletalMesh|GetAnimInstance (Variables|Character|GetMesh))))
  (if (Variables|/Game/Characters/Work_Sami/Anims/DevourerAnim/DevourerAnim.DevourerAnim_C|GetisTazed _asdevourer_anim)
    (AI|Navigation|StopMovement (AI|GetAIController self))
    (if (Variables|Default|GetPlayedTazedOnce)
      _
      (else
        (Variables|Default|SetPlayedTazedOnce true)
        (Audio|Components|Audio|Stop (Variables|Default|GetDevourerAudio))
        (Audio|PlaySoundatLocation (Variables|Default|GetTazedSound) (Transformation|GetActorLocation self) "0, 0, 0" 1.0 1.0 0.0 0 0 0 0)))
    (Variables|Default|SetIsMoving true)
    (Variables|/Script/Engine.SkeletalMeshComponent|SetGlobalAnimRateScale (Variables|Character|GetMesh) 1.0)
    (else
      (Variables|Default|SetPlayedTazedOnce false)
      (bind (_outhit _returnvalue_3) (Collision|SphereTraceForObjects _returnvalue_2 _returnvalue_2 1.5e+03 (Utilities|Array|MakeArray "ObjectTypeQuery3") false 0 "None"))
      (if _returnvalue_3
        (Utilities|Casting|CastToBP_ThirdPersonCharacter (.HitActor (Collision|BreakHitResult _outhit))
          (:then
            (if (Class|PrimitiveComponent|WasRecentlyRendered (Variables|Character|GetMesh) 0.1)
              (if (== (Variables|/Script/Engine.AudioComponent|GetSound _devoureraudio_2) (Variables|Default|GetChaseSound))
                _
                (else
                  (Audio|Components|Audio|Stop _devoureraudio_2)))
              (Audio|Components|Audio|SetSound _devoureraudio_2 (Variables|Default|GetChaseSound))
              (Audio|Components|Audio|Play _devoureraudio_2 0.0)
              (if (Variables|Default|GetisMoving)
                (bind _returnvalue_4 (Collision|LineTraceByChannel (Transformation|GetActorLocation self) (Camera|GetCameraLocation (Game|GetPlayerCameraManager 0)) "TraceTypeQuery1" false 0 "None"))
                (if (not _returnvalue_4)
                  (Variables|/Script/Engine.SkeletalMeshComponent|SetGlobalAnimRateScale (Variables|Character|GetMesh) 0.0)
                  (AI|Navigation|StopMovement (Pawn|GetController))
                  (Variables|Default|SetIsMoving false)
                  (Variables|/Script/Engine.SkeletalMeshComponent|SetGlobalAnimRateScale (Variables|Character|GetMesh) 0.0)
                  (Variables|/Script/Engine.MovementComponent|SetVelocity (Variables|Character|GetCharacterMovement) "0, 0, 0")))
              (else
                (AI|Navigation|SimpleMovetoLocation (Pawn|GetController) (Transformation|GetActorLocation (Game|GetPlayerCharacter 0)))
                (Variables|Default|SetIsMoving true)
                (Variables|/Script/Engine.SkeletalMeshComponent|SetGlobalAnimRateScale (Variables|Character|GetMesh) 1.0))))
          (:CastFailed
            (if (Audio|Components|Audio|IsPlaying _devoureraudio) :!label _label
              (if (== (Variables|/Script/Engine.AudioComponent|GetSound _devoureraudio) (Variables|Default|GetChaseSound))
                (Audio|Components|Audio|Stop _devoureraudio))
              (else
                (Audio|Components|Audio|SetSound _devoureraudio "/Game/Characters/Work_Sami/Sounds/Devourer/Devourer_Idle_BreathingRandom.Devourer_Idle_BreathingRandom")
                (Audio|Components|Audio|Play _devoureraudio 0.0)))
            (if (Variables|Default|GetreachedDestination)
              (AI|AIMoveTo self _randomlocation 0 0.0 false
                (:then
                  (Variables|Default|SetreachedDestination false)
                  (Variables|Default|SetIsMoving true)
                  (Variables|/Script/Engine.SkeletalMeshComponent|SetGlobalAnimRateScale (Variables|Character|GetMesh) 1.0)
                  (Utilities|String|LogString "DRD")))
              (elif (<= (Math|Vector|Distance(Vector) _randomlocation (Transformation|GetActorLocation)) 1.5e+02)
                (Utilities|Casting|CastToDevourerAnim (Components|SkeletalMesh|GetAnimInstance (Variables|Character|GetMesh)))
                (Variables|Default|SetreachedDestination true)
                (Variables|Default|SetIsMoving true)
                (Variables|/Script/Engine.SkeletalMeshComponent|SetGlobalAnimRateScale (Variables|Character|GetMesh) 1.0)
                (Development|PrintString "RD")))))
        (else
          (goto _label))))))

(fn ConstructionScript)