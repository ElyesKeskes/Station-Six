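; BP_ItemData is an inventory item data class for examinable items in a horror game, with empty hooks for construct, examine, collect and reset.
; LoadfromDT extends the parent loader, copying mesh or actor class, interaction box, rotation offsets and collectability from the data.
; Discard runs the parent logic, then optionally has BP_HorrorGameState spawn a dropped item at the character's feet, carrying quantity, GUID and checkpoint data.
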(event Custom|OnConstruct)

(event Custom|OnExamine)

(event Custom|OnCollected
  (params (PlayerController :type Player%20Controller%20Object%20Reference) (ExaminableObjectRef :type Object%20Object%20Reference)))

(event Custom|OnReset)

(event EventLoadfromDT
  (params (BaseData :type Inventory%20Item%20DT%20Base%20Struct%20Structure))
  (bind (_examinablemesh _examiningrotationoffset _rotationoffset _interactiveboxscale _canbecollected) (Utilities|Struct|BreakInventoryItemDTBase_Struct BaseData))
  (bind (_staticmesh _skeletalmesh _actorclass) (Utilities|Struct|BreakExaminableItemMeshDT_Struct _examinablemesh))
  (|CallParentFunction BaseData)
  (Variables|ExaminableItem|SetStaticMesh _staticmesh)
  (Variables|ExaminableItem|SetSkeletalMesh _skeletalmesh)
  (Variables|ExaminableItem|SetActorClass (Utilities|ResolveSoftReference _actorclass))
  (Variables|Examinable|SetInteractiveBoxScale _interactiveboxscale)
  (Variables|Examinable|SetRotationOffset _rotationoffset)
  (Variables|Examinable|SetExaminingRotationOffset _examiningrotationoffset)
  (Variables|Examinable|SetCanBeCollected _canbecollected))

(fn OnInteractAction
  (return "NewEnumerator0"))

(fn Discard
  (bind _droptheitemondiscard (Variables|Default|GetDropTheItemOnDiscard))
  (bind _success (|CallParentFunction))
  (if _success
    (Utilities|FlowControl|Sequence
      (:then_0
        (if _droptheitemondiscard
          ;[0.2 0.2 0.2 0.2] Spawn Dropped Item
          (bind _asbp_horror_game_state (Utilities|Casting|CastToBP_HorrorGameState (Variables|Default|GetGameState)))
          (bind _ascharacter (Utilities|Casting|CastToCharacter (Pawn|GetControlledPawn (Default|GetPlayerController _asbp_horror_game_state))))
          (bind _returnvalue (Game|ConstructObjectfromClass self "/Game/HorrorMechanics/Blueprint/SaveSystem/BP_CheckpointDataContainer.BP_CheckpointDataContainer_C" (Utilities|Struct|MakeGenericDataContainer_Struct)))
          (bind (__checkpointdatamanager _savestruct) (CallFunction|GetCheckpointData _returnvalue))
          (Utilities|IsValid __checkpointdatamanager
            (:Is%20Valid
              (LocalVariables|SetItemData (Variables|/Game/HorrorMechanics/Blueprint/SaveSystem/BP_CheckpointDataContainer.BP_CheckpointDataContainer_C|GetDataStruct __checkpointdatamanager)))
            (:Is%20Not%20Valid
              (LocalVariables|SetItemData _savestruct)))
          (Default|SpawnDroppedItem _asbp_horror_game_state (Math|Transform|MakeTransform (- (Transformation|GetActorLocation _ascharacter) (Math|Vector|MakeVector 0.0 0.0 (Variables|/Script/Engine.CapsuleComponent|GetCapsuleHalfHeight (Variables|/Script/Engine.Character|GetCapsuleComponent _ascharacter))))) 0 (Variables|Default|GetQuantity) (LocalVariables|GetItemData) (Variables|Default|GetGUID))))
      (:then_1
        (return _success _droptheitemondiscard)))))