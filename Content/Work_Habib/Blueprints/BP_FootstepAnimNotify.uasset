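; Animation notify that plays surface-dependent footstep sounds for CH_PlayerCharacter and reports them as noise events for AI hearing.
; A downward visibility trace that ignores player characters finds the surface type, which keys into the character's FootstepSoundsMap.
; It plays a random sound from that entry with slight pitch variation, falling back to the SurfaceType2 entry for unmapped surfaces.
; No sound or noise occurs when the trace misses.
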(fn ReceivedNotify
  (params (MeshComp :type Skeletal%20Mesh%20Component%20Object%20Reference) (Animation :type Anim%20Sequence%20Base%20Object%20Reference) (EventReference :type Anim%20Notify%20Event%20Reference%20Structure%20%28by%20ref%29))
  (bind _returnvalue (Components|GetOwner MeshComp))
  (bind _returnvalue_2 (Math|Random|RandomFloatinRange 0.9 1.1))
  (bind _returnvalue_3 (Transformation|GetActorLocation _returnvalue))
  (bind _outactors (Actor|GetAllActorsOfClass "/Game/HorrorMechanics/ExampleAssets/Blueprint/Characters/CH_PlayerCharacter.CH_PlayerCharacter_C"))
  (bind (_outhit _returnvalue_4) (Collision|LineTraceByChannel _returnvalue_3 (+ _returnvalue_3 (* (Transformation|GetActorUpVector _returnvalue) -2e+02)) "TraceTypeQuery1" false _outactors "None"))
  (if _returnvalue_4
    (bind _asch_player_character (Utilities|Casting|CastToCH_PlayerCharacter _returnvalue))
    (if (.ReturnValue (Utilities|Map|Find (Variables|/Game/HorrorMechanics/ExampleAssets/Blueprint/Characters/CH_PlayerCharacter.CH_PlayerCharacter_C|GetFootstepSoundsMap _asch_player_character) (Collision|GetSurfaceType _outhit)))
      (Audio|PlaySoundatLocation (.OutItem (Utilities|Array|Random (Variables|/Game/Work_Habib/DataAssets/FootstepDataAsset.FootstepDataAsset_C|GetFootstepSounds (.Value (Utilities|Map|Find (Variables|/Game/HorrorMechanics/ExampleAssets/Blueprint/Characters/CH_PlayerCharacter.CH_PlayerCharacter_C|GetFootstepSoundsMap _asch_player_character) (Collision|GetSurfaceType _outhit)))))) _returnvalue_3 "0, 0, 0" 0.4 _returnvalue_2 0.0 0 0 0 0)
      (else
        (Audio|PlaySoundatLocation (.OutItem (Utilities|Array|Random (Variables|/Game/Work_Habib/DataAssets/FootstepDataAsset.FootstepDataAsset_C|GetFootstepSounds (.Value (Utilities|Map|Find (Variables|/Game/HorrorMechanics/ExampleAssets/Blueprint/Characters/CH_PlayerCharacter.CH_PlayerCharacter_C|GetFootstepSoundsMap _asch_player_character) "SurfaceType2"))))) _returnvalue_3 "0, 0, 0" 0.4 _returnvalue_2 0.0 0 0 0 0)))
    (Class|AISenseHearing|ReportNoiseEvent _returnvalue_3 1.0 0 5e+02 "None")
    (return false)))