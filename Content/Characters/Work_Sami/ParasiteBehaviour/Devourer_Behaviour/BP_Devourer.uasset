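; BP_Devourer is an enemy character that freezes when the player sees it and hunts them when unseen.
; Each tick, a sphere trace looks for the player; recent rendering plus an unblocked trace to the camera halts movement and animation.
; Off screen, it moves to the player and deals cooldown-limited damage.
; Otherwise it wanders with breathing audio, while a tazed flag from DevourerAnim stops it and overrides this behaviour.
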(event EventTick
  (params (DeltaSeconds :type Float%20%28single-precision%29))
  (bind _returnvalue (Transformation|GetActorLocation))
  (bind _self self)
  (bind _self_2 self)
  (bind _devoureraudio (Variables|Default|GetDevourerAudio))
  (bind _devoureraudio_2 (Variables|Default|GetDevourerAudio))
  (bind _randomlocation (AI|Navigation|GetRandomReachablePointinRadius _returnvalue 1.5e+03 0 0))
  (bind _returnvalue_2 (Transformation|GetActorLocation _self_2))
  (bind _asdevourer_anim (Utilities|Casting|CastToDevourerAnim (Components|SkeletalMesh|GetAnimInstance (Variables|Character|GetMesh))))
  (if (Variables|/Game/Characters/Work_Sami/Anims/DevourerAnim/DevourerAnim.DevourerAnim_C|GetisTazed _asdevourer_anim)
    (AI|Navigation|StopMovement (AI|GetAIController self))
    (if (Variables|Default|GetPlayedTazedOnce)
      _
      (else
        (Variables|Default|SetPlayedTazedOnce true)
        (Audio|Components|Audio|Stop (Variables|Default|GetDevourerAudio))
        (Audio|PlaySoundatLocation (Variables|Default|GetTazedSound) (Transformation|GetActorLocation self) "0, 0, 0" 1.0 1.0 0.0 0 0 0 0)))
    (Variables|Default|SetIsMoving true)
    (Variables|/Script/Engine.SkeletalMeshComponent|SetGlobalAnimRateScale (Variables|Character|GetMesh) 1.0)
    (else
      (Variables|Default|SetPlayedTazedOnce false)
      (bind (_outhits _returnvalue_3) (Collision|MultiSphereTraceForObjects _returnvalue_2 _returnvalue_2 1.5e+03 (Utilities|Array|MakeArray "ObjectTypeQuery3") false 0 "None"))
      (for _array_element _outhits
        (if _returnvalue_3
          (Utilities|Casting|CastToCH_PlayerCharacter (.HitActor (Collision|BreakHitResult _array_element))
            (:then
              (if (Class|PrimitiveComponent|WasRecentlyRendered (Variables|Character|GetMesh) 0.1)
                (AI|AIMoveTo _self "0, 0, 0" _self 5.0 false
                  (:then
                    (if (== (Variables|/Script/Engine.AudioComponent|GetSound _devoureraudio_2) (Variables|Default|GetChaseSound))
                      _
                      (else
                        (Audio|Components|Audio|Stop _devoureraudio_2)))
                    (Audio|Components|Audio|SetSound _devoureraudio_2 (Variables|Default|GetChaseSound))
                    (Audio|Components|Audio|Play _devoureraudio_2 0.0)
                    (if (Variables|Default|GetisMoving)
                      (bind _returnvalue_4 (Collision|LineTraceByChannel (Transformation|GetActorLocation self) (Camera|GetCameraLocation (Game|GetPlayerCameraManager 0)) "TraceTypeQuery1" false 0 "None"))
                      (if (not _returnvalue_4)
                        (Variables|/Script/Engine.SkeletalMeshComponent|SetGlobalAnimRateScale (Variables|Character|GetMesh) 0.0)
                        (AI|Navigation|StopMovement (Pawn|GetController))
                        (Variables|Default|SetIsMoving false)
                        (Variables|/Script/Engine.SkeletalMeshComponent|SetGlobalAnimRateScale (Variables|Character|GetMesh) 0.0)
                        (Variables|/Script/Engine.MovementComponent|SetVelocity (Variables|Character|GetCharacterMovement) "0, 0, 0")))))
                (else
                  (AI|AIMoveTo self "0, 0, 0" (Game|GetPlayerCharacter 0) 1.5e+02 false
                    (:OnSuccess
                      (Variables|Default|SetIsMoving true)
                      (Variables|/Script/Engine.SkeletalMeshComponent|SetGlobalAnimRateScale (Variables|Character|GetMesh) 1.0)
                      (if (Variables|Default|GetCanAttack?)
                        (Variables|Default|SetCanAttack? false)
                        (Animation|PlayAnimMontage "/Game/Characters/Work_Sami/Anims/DevourerAnim/idleMontage.idleMontage" 1.0 "None")
                        (Game|Damage|ApplyDamage (Game|Player|GetPlayerPawn 0) 7e+01 (Pawn|GetController) self)
                        (Utilities|FlowControl|Delay 2.0)
                        (Variables|Default|SetCanAttack? true)))))))
            (:CastFailed
              (if (Audio|Components|Audio|IsPlaying _devoureraudio) :!label _label
                (if (== (Variables|/Script/Engine.AudioComponent|GetSound _devoureraudio) (Variables|Default|GetChaseSound))
                  (Audio|Components|Audio|Stop _devoureraudio))
                (else
                  (Audio|Components|Audio|SetSound _devoureraudio "/Game/Characters/Work_Sami/Sounds/Devourer/Devourer_Idle_BreathingRandom.Devourer_Idle_BreathingRandom")
                  (Audio|Components|Audio|Play _devoureraudio 0.0)))
              (if (Variables|Default|GetreachedDestination)
                (AI|AIMoveTo self _randomlocation 0 0.0 false
                  (:then
                    (Variables|Default|SetreachedDestination false)
                    (Variables|Default|SetIsMoving true)
                    (Variables|/Script/Engine.SkeletalMeshComponent|SetGlobalAnimRateScale (Variables|Character|GetMesh) 1.0)))
                (elif (<= (Math|Vector|Distance(Vector) _randomlocation (Transformation|GetActorLocation)) 1.5e+02)
                  (Utilities|Casting|CastToDevourerAnim (Components|SkeletalMesh|GetAnimInstance (Variables|Character|GetMesh)))
                  (Variables|Default|SetreachedDestination true)
                  (Variables|Default|SetIsMoving true)
                  (Variables|/Script/Engine.SkeletalMeshComponent|SetGlobalAnimRateScale (Variables|Character|GetMesh) 1.0)))))
          (else
            (goto _label))))
      (if _returnvalue_3
        (Utilities|Casting|CastToCH_PlayerCharacter (.HitActor (Collision|BreakHitResult _array_element))
          (:then
            (if (Class|PrimitiveComponent|WasRecentlyRendered (Variables|Character|GetMesh) 0.1)
              (AI|AIMoveTo _self "0, 0, 0" _self 5.0 false
                (:then
                  (if (== (Variables|/Script/Engine.AudioComponent|GetSound _devoureraudio_2) (Variables|Default|GetChaseSound))
                    _
                    (else
                      (Audio|Components|Audio|Stop _devoureraudio_2)))
                  (Audio|Components|Audio|SetSound _devoureraudio_2 (Variables|Default|GetChaseSound))
                  (Audio|Components|Audio|Play _devoureraudio_2 0.0)
                  (if (Variables|Default|GetisMoving)
                    (bind _returnvalue_5 (Collision|LineTraceByChannel (Transformation|GetActorLocation self) (Camera|GetCameraLocation (Game|GetPlayerCameraManager 0)) "TraceTypeQuery1" false 0 "None"))
                    (if (not _returnvalue_5)
                      (Variables|/Script/Engine.SkeletalMeshComponent|SetGlobalAnimRateScale (Variables|Character|GetMesh) 0.0)
                      (AI|Navigation|StopMovement (Pawn|GetController))
                      (Variables|Default|SetIsMoving false)
                      (Variables|/Script/Engine.SkeletalMeshComponent|SetGlobalAnimRateScale (Variables|Character|GetMesh) 0.0)
                      (Variables|/Script/Engine.MovementComponent|SetVelocity (Variables|Character|GetCharacterMovement) "0, 0, 0")))))
              (else
                (AI|AIMoveTo self "0, 0, 0" (Game|GetPlayerCharacter 0) 1.5e+02 false
                  (:OnSuccess
                    (Variables|Default|SetIsMoving true)
                    (Variables|/Script/Engine.SkeletalMeshComponent|SetGlobalAnimRateScale (Variables|Character|GetMesh) 1.0)
                    (if (Variables|Default|GetCanAttack?)
                      (Variables|Default|SetCanAttack? false)
                      (Animation|PlayAnimMontage "/Game/Characters/Work_Sami/Anims/DevourerAnim/idleMontage.idleMontage" 1.0 "None")
                      (Game|Damage|ApplyDamage (Game|Player|GetPlayerPawn 0) 7e+01 (Pawn|GetController) self)
                      (Utilities|FlowControl|Delay 2.0)
                      (Variables|Default|SetCanAttack? true)))))))
          (:CastFailed
            (if (Audio|Components|Audio|IsPlaying _devoureraudio) :!label _label_2
              (if (== (Variables|/Script/Engine.AudioComponent|GetSound _devoureraudio) (Variables|Default|GetChaseSound))
                (Audio|Components|Audio|Stop _devoureraudio))
              (else
                (Audio|Components|Audio|SetSound _devoureraudio "/Game/Characters/Work_Sami/Sounds/Devourer/Devourer_Idle_BreathingRandom.Devourer_Idle_BreathingRandom")
                (Audio|Components|Audio|Play _devoureraudio 0.0)))
            (if (Variables|Default|GetreachedDestination)
              (AI|AIMoveTo self _randomlocation 0 0.0 false
                (:then
                  (Variables|Default|SetreachedDestination false)
                  (Variables|Default|SetIsMoving true)
                  (Variables|/Script/Engine.SkeletalMeshComponent|SetGlobalAnimRateScale (Variables|Character|GetMesh) 1.0)))
              (elif (<= (Math|Vector|Distance(Vector) _randomlocation (Transformation|GetActorLocation)) 1.5e+02)
                (Utilities|Casting|CastToDevourerAnim (Components|SkeletalMesh|GetAnimInstance (Variables|Character|GetMesh)))
                (Variables|Default|SetreachedDestination true)
                (Variables|Default|SetIsMoving true)
                (Variables|/Script/Engine.SkeletalMeshComponent|SetGlobalAnimRateScale (Variables|Character|GetMesh) 1.0)))))
        (else
          (goto _label_2))))))

(fn ConstructionScript)