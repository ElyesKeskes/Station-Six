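; Camera modifier that applies a blurred, darkened, vignetted screen effect in the horror game.
; It overrides post-process settings with reduced color gain and depth of field at a focal distance, blended by the modifier's alpha, and leaves view location, rotation and FOV untouched.
; The game state's engine version selects aperture-based depth of field for 4.23 and later, or the Gaussian method for older versions.
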(fn BlueprintModifyPostProcess
  (params (DeltaTime :type Float%20%28single-precision%29))
  (bind _returnvalue (Math|Vector4|MakeVector4 0.7 0.7 0.7 1.0))
  (bind _focaldistance (Variables|Default|GetFocalDistance))
  (return (Variables|CameraModifier|GetAlpha) (select (>= (Variables|/Game/HorrorMechanics/Blueprint/Game/BP_HorrorGameState.BP_HorrorGameState_C|GetUE4Version (CallFunction|GetHorrorGameState)) 423) (Utilities|Struct|MakePostProcessSettings _returnvalue -5e+02 1e+01 1.0 _focaldistance) (Utilities|Struct|MakePostProcessSettings _returnvalue -5e+02 1.0 1.0 _focaldistance 1.5e+02 0.0 1e+01 "DOFM_Gaussian"))))

(fn BlueprintModifyCamera
  (params (DeltaTime :type Float%20%28single-precision%29) (ViewLocation :type Vector :default "0, 0, 0") (ViewRotation :type Rotator :default "0, 0, 0") (FOV :type Float%20%28single-precision%29))
  (return ViewLocation ViewRotation FOV))