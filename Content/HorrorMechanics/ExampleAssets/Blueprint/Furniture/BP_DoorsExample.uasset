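; BP_DoorsExample is an example furniture Blueprint from HorrorMechanics with two cabinet doors and two drawers.
; SetupComponents configures the doors with a shared opening angle but different open axes, and the drawers with a shared length and axis.
; BeginPlay runs the parent logic, then initializes each door and drawer.
; The setup and initialization functions are not defined in these graphs, which only wire the components into them.
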(event EventBeginPlay
  (|CallParentFunction)
  (CallFunction|InitializeCabinetDoor (Variables|Components|GetLeftDoor))
  (CallFunction|InitializeCabinetDoor (Variables|Components|GetRightDoor))
  (CallFunction|InitializeDrawer (Variables|Components|GetLeftDrawer))
  (CallFunction|InitializeDrawer (Variables|Components|GetRightDrawer)))

(event EventTick
  (params (DeltaSeconds :type Float%20%28single-precision%29))
  (|CallParentFunction DeltaSeconds) ; This node is disabled and will not be called.\nDrag off pins to build functionality.
)

(event EventSetupComponents
  (bind _drawerslength (Variables|Default|GetDrawersLength))
  (bind _cabinetdooropeningangle (Variables|Default|GetCabinetDoorOpeningAngle))
  (CallFunction|SetupCabinetDoor (Variables|Components|GetLeftDoor) _cabinetdooropeningangle "NewEnumerator2")
  (CallFunction|SetupCabinetDoor (Variables|Components|GetRightDoor) _cabinetdooropeningangle "NewEnumerator5")
  (CallFunction|SetupDrawer (Variables|Components|GetLeftDrawer) "NewEnumerator0" _drawerslength)
  (CallFunction|SetupDrawer (Variables|Components|GetRightDrawer) "NewEnumerator0" _drawerslength))

(fn ConstructionScript
  (|CallParentFunction))