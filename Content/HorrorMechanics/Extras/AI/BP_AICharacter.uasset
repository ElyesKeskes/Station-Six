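; Enemy AI character for a horror game that opens doors in its path and attacks the player in melee.
; Tick traces forward, opens closed doors while pausing movement for a montage, and launches the player through open doorways when both occupy the door's areas.
; Attack halts pathing and plays a montage, while a separate DealDamage event sphere-traces from the spine socket to hurt the player.
; Incoming point damage is only printed as debug text.
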(event Custom|Attack
  (Class|NavMovementComponent|StopMovementKeepPathing (Variables|Character|GetCharacterMovement))
  (Variables|Default|SetAttacking true)
  (Utilities|FlowControl|Sequence
    (:then_0
      (Animation|Montage|PlayMontage (Variables|Character|GetMesh) "/Game/HorrorMechanics/Extras/AI/Animations/AM_Attack.AM_Attack" 1.25
        (:OnCompleted
          _)
        (:OnInterrupted
          _))
      (Variables|Default|SetAttacking false))))

(event Custom|DealDamage
  (bind _mesh (Variables|Character|GetMesh))
  (bind _returnvalue (Transformation|GetSocketTransform _mesh "spine_02" "RTS_World"))
  (bind (_outhit _returnvalue_2) (Collision|SphereTraceByChannel (.location _returnvalue) (+ (.location _returnvalue) (* (Math|Vector|GetRightVector (.rotation _returnvalue)) 1.5e+02)) 3e+01 "TraceTypeQuery1" false 0 "None"))
  (if _returnvalue_2
    (bind _ascharacter (Utilities|Casting|CastToCharacter (.HitActor (Collision|BreakHitResult _outhit))))
    (Utilities|Casting|CastToPlayerController (Pawn|GetController _ascharacter))
    (Game|Damage|ApplyDamage (Game|GetPlayerCharacter 0) 1e+01 (Pawn|GetController) self)))

(event EventBeginPlay)

(event Collision|EventActorBeginOverlap
  (params (OtherActor :type Actor%20Object%20Reference)))

(event EventTick
  (params (DeltaSeconds :type Float%20%28single-precision%29))
  (bind _returnvalue (Transformation|GetActorLocation))
  (bind _returnvalue_2 (Game|GetPlayerCharacter 0))
  (bind _self self)
  (bind _charactermovement (Variables|Character|GetCharacterMovement))
  (Utilities|FlowControl|Sequence
    (:then_0
      (bind (_outhit _returnvalue_3) (Collision|LineTraceByChannel _returnvalue (+ _returnvalue (* (Transformation|GetActorForwardVector) 1e+02)) "TraceTypeQuery1" false 0 "None"))
      (if _returnvalue_3
        (bind _asbp_door_abstract_class (Utilities|Casting|CastToBP_DoorAbstractClass (.HitActor (Collision|BreakHitResult _outhit))))
        (if (Variables|/Game/HorrorMechanics/Blueprint/Doors/BP_DoorAbstractClass.BP_DoorAbstractClass_C|GetIsClosed _asbp_door_abstract_class)
          (Default|Interaction _asbp_door_abstract_class)
          (Class|NavMovementComponent|StopMovementKeepPathing _charactermovement)
          (Pawn|Components|CharacterMovement|DisableMovement _charactermovement)
          (Variables|Default|SetInteractionTime (Utilities|Time|GetTimeSeconds))
          (Animation|Montage|PlayMontage (Variables|Character|GetMesh) "/Game/HorrorMechanics/Extras/AI/Animations/AM_Interact.AM_Interact"
            (:OnCompleted
              _)
            (:OnInterrupted
              _))
          (Pawn|Components|CharacterMovement|SetMovementMode _charactermovement "MOVE_Walking" 0)
          (elif (Utilities|Enum|Equal(Enum) (Variables|/Script/Engine.CharacterMovementComponent|GetMovementMode _charactermovement) "MOVE_Walking")
            (if (or (== (Variables|/Game/HorrorMechanics/Blueprint/Doors/BP_DoorAbstractClass.BP_DoorAbstractClass_C|GetState _asbp_door_abstract_class) -1) (== (Variables|/Game/HorrorMechanics/Blueprint/Doors/BP_DoorAbstractClass.BP_DoorAbstractClass_C|GetState _asbp_door_abstract_class) 0))
              ;[0.2 0.2 0.2 0.2] Pushes player on the other side of door
              (if (and (Collision|IsOverlappingActor (Variables|/Game/HorrorMechanics/Blueprint/Doors/BP_DoorAbstractClass.BP_DoorAbstractClass_C|GetOpeningAreaComp _asbp_door_abstract_class) _self :!class /Script/Engine.PrimitiveComponent) (Collision|IsOverlappingActor (Variables|/Game/HorrorMechanics/Blueprint/Doors/BP_DoorAbstractClass.BP_DoorAbstractClass_C|GetCrossingAreaComp _asbp_door_abstract_class) _returnvalue_2 :!class /Script/Engine.PrimitiveComponent))
                (Character|LaunchCharacter _returnvalue_2 (+ (* (Transformation|GetActorRightVector _asbp_door_abstract_class) -5e+02) "0, 0,10.000000") true true)
                (elif (and (Collision|IsOverlappingActor (Variables|/Game/HorrorMechanics/Blueprint/Doors/BP_DoorAbstractClass.BP_DoorAbstractClass_C|GetOpeningAreaComp _asbp_door_abstract_class) _returnvalue_2 :!class /Script/Engine.PrimitiveComponent) (Collision|IsOverlappingActor (Variables|/Game/HorrorMechanics/Blueprint/Doors/BP_DoorAbstractClass.BP_DoorAbstractClass_C|GetCrossingAreaComp _asbp_door_abstract_class) _self :!class /Script/Engine.PrimitiveComponent))
                  (Character|LaunchCharacter _returnvalue_2 (+ (* (Transformation|GetActorRightVector _asbp_door_abstract_class) 5e+02) "0, 0,10.000000") true true))))))))))

(event Game|Damage|EventPointDamage
  (params (Damage :type Float%20%28single-precision%29) (DamageType :type Damage%20Type%20Object%20Reference) (HitLocation :type Vector :default "0, 0, 0") (HitNormal :type Vector :default "0, 0, 0") (HitComponent :type Primitive%20Component%20Object%20Reference) (BoneName :type Name :default "None") (ShotFromDirection :type Vector :default "0, 0, 0") (InstigatedBy :type Controller%20Object%20Reference) (DamageCauser :type Actor%20Object%20Reference) (HitInfo :type Hit%20Result%20Structure%20%28by%20ref%29))
  (Development|PrintString (Utilities|String|Append "DAMAGED: " (Utilities|String|ToString(Float) Damage) " to: " (Utilities|String|ToString(Name) BoneName) " of " (Utilities|GetObjectName self)) true true "(R=1.000000,G=0.182528,B=0.052770,A=1.000000)"))

(fn ConstructionScript)