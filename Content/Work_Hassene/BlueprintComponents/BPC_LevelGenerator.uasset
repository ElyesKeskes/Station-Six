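; Actor component that procedurally builds a level from random rooms on a grid, then populates it.
; Starting from the start room and elevator, it grows a queue of origin rooms through compatible sockets until the room cap, then plugs unused sockets.
; It then removes off-map reference rooms, places puzzle items, batteries and ammo at type-filtered spawn points, and spawns doors at connected sockets.
; Enemy spawn points are filtered, but enemy spawning is disconnected.
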(event EventProcessNextOriginRoominQueue
  (bind _queuedoriginrooms (Variables|StatusVariables|GetQueuedOriginRooms))
  ;[0 0.07001 1 0.18] Level layout generation
  (if (< (Variables|StatusVariables|GetSpawnedRoomsNumber) (Variables|GenerationParameters|GetMaxRoomNumber))
    (bind _output_get (Variables|CurrentConnectionLoop|SetOriginRoom (Utilities|Array|Get(acopy) _queuedoriginrooms (Utilities|Array|LastIndex _queuedoriginrooms))))
    (Utilities|IsValid _output_get
      (:Is%20Valid
        (if (Utilities|Array|IsNotEmpty (Variables|/Game/Work_Hassene/Prefabs/Master/BPP_BaseRoom.BPP_BaseRoom_C|GetPossibleRoomConnections (Variables|CurrentConnectionLoop|GetOriginRoom)))
          (Variables|CurrentConnectionLoop|SetTempPossibleRoomConnection (Utilities|Array|Get(acopy) (Variables|/Game/Work_Hassene/Prefabs/Master/BPP_BaseRoom.BPP_BaseRoom_C|GetPossibleRoomConnections (Variables|CurrentConnectionLoop|GetOriginRoom)) (Utilities|Array|LastIndex (Variables|/Game/Work_Hassene/Prefabs/Master/BPP_BaseRoom.BPP_BaseRoom_C|GetPossibleRoomConnections (Variables|CurrentConnectionLoop|GetOriginRoom)))))
          (Utilities|FlowControl|Sequence
            (:then_0
              (Variables|CurrentConnectionLoop|SetOriginRoomSocket (.existingsocket (Variables|CurrentConnectionLoop|GetTempPossibleRoomConnection)))
              (Variables|CurrentConnectionLoop|SetOriginRoomSocketIndex (.index (Variables|CurrentConnectionLoop|GetOriginRoomSocket))))
            (:then_1
              (Variables|CurrentConnectionLoop|SetTempPossibleRoomDataArray (.possibleroomdata (Variables|CurrentConnectionLoop|GetTempPossibleRoomConnection))))
            (:then_2
              (Variables|CurrentConnectionLoop|SetRandomSelectedPossibleRoomDataIndex (.OutIndex (Utilities|Array|Random (Variables|CurrentConnectionLoop|GetTempPossibleRoomDataArray))))
              (Utilities|FlowControl|Sequence
                (:then_0
                  (Variables|CurrentConnectionLoop|SetSelectedDerivedRoom (.possibleroom (Utilities|Array|Get(acopy) (Variables|CurrentConnectionLoop|GetTempPossibleRoomDataArray) (Variables|CurrentConnectionLoop|GetRandomSelectedPossibleRoomDataIndex)))))
                (:then_1
                  (Variables|CurrentConnectionLoop|SetTempPossibleRoomsCompatibleSocketsArray (.possibleroomscompatiblesockets (Utilities|Array|Get(acopy) (Variables|CurrentConnectionLoop|GetTempPossibleRoomDataArray) (Variables|CurrentConnectionLoop|GetRandomSelectedPossibleRoomDataIndex)))))
                (:then_2
                  (Variables|CurrentConnectionLoop|SetRandomSelectedPossibleRoomCompatibleSocketIndex (.OutIndex (Utilities|Array|Random (Variables|CurrentConnectionLoop|GetTempPossibleRoomsCompatibleSocketsArray))))
                  (Variables|CurrentConnectionLoop|SetDerivedRoomSocket (Utilities|Array|Get(acopy) (Variables|CurrentConnectionLoop|GetTempPossibleRoomsCompatibleSocketsArray) (Variables|CurrentConnectionLoop|GetRandomSelectedPossibleRoomCompatibleSocketIndex)))
                  (Variables|CurrentConnectionLoop|SetRoomToConnectAnchorCoordinates (Utilities|Array|Get(acopy) (.possibleroomsanchorpoints (Utilities|Array|Get(acopy) (Variables|CurrentConnectionLoop|GetTempPossibleRoomDataArray) (Variables|CurrentConnectionLoop|GetRandomSelectedPossibleRoomDataIndex))) (Variables|CurrentConnectionLoop|GetRandomSelectedPossibleRoomCompatibleSocketIndex)))
                  (Utilities|FlowControl|Sequence
                    (:then_0
                      ;;[0.9387 0.5512 1] Spawning Room
                      (bind _returnvalue (Game|SpawnActorfromClass (Utilities|GetClass (Variables|CurrentConnectionLoop|GetSelectedDerivedRoom)) (Math|Transform|MakeTransform (Class|GridActorComponent|GetSpaceCenterWorldLocation (Variables|Default|GetGrid) (Variables|CurrentConnectionLoop|GetRoomToConnectAnchorCoordinates) (Variables|/Game/Work_Hassene/Prefabs/Master/BPP_BaseRoom.BPP_BaseRoom_C|GetSize (Variables|CurrentConnectionLoop|GetSelectedDerivedRoom))) "0, 0, 0" "1.000000,1.000000,1.000000") "AdjustIfPossibleButDontSpawnIfColliding" "MultiplyWithRoot" 0 0))
                      (bind _output_get_2 (Variables|StatusVariables|SetLastSpawnedDerivedRoom _returnvalue))
                      (Variables|/Game/Work_Hassene/Prefabs/Master/BPP_BaseRoom.BPP_BaseRoom_C|SetAnchorCoordinates _output_get_2 (Variables|CurrentConnectionLoop|GetRoomToConnectAnchorCoordinates))
                      (Default|SetupRoom (Variables|StatusVariables|GetLastSpawnedDerivedRoom)))
                    (:then_1
                      ;;[1 0.5573 0.5573] Updating grid
                      (Class|GridActorComponent|MarkSpaceOccupied (Variables|Default|GetGrid) (Variables|CurrentConnectionLoop|GetRoomToConnectAnchorCoordinates) (Variables|/Game/Work_Hassene/Prefabs/Master/BPP_BaseRoom.BPP_BaseRoom_C|GetSize (Variables|StatusVariables|GetLastSpawnedDerivedRoom)))
                      (Utilities|Array|AddUnique (Variables|StatusVariables|GetSpawnedRooms) (Variables|StatusVariables|GetLastSpawnedDerivedRoom))
                      (Math|Integer|IncrementInt (Variables|StatusVariables|GetSpawnedRoomsNumber)
                        (:%20%20
                          (Utilities|Array|AddUnique (Variables|StatusVariables|GetQueuedOriginRooms) (Variables|StatusVariables|GetLastSpawnedDerivedRoom)))))
                    (:then_2
                      ;;[0.4773 0.4503 1 0.446] Updating sockets and possible connections in each room in the established connection
                      (Utilities|FlowControl|Sequence
                        (:then_0
                          (Default|UpdateSocketsandPossibleConnections (Variables|CurrentConnectionLoop|GetOriginRoom) (Variables|CurrentConnectionLoop|GetOriginRoomSocketIndex) (Variables|StatusVariables|GetLastSpawnedDerivedRoom) (Variables|CurrentConnectionLoop|GetOriginRoomSocket))
                          (Default|AssemblePossibleRoomConnections (Variables|CurrentConnectionLoop|GetOriginRoom)))
                        (:then_1
                          (Default|UpdateSocketsandPossibleConnections (Variables|StatusVariables|GetLastSpawnedDerivedRoom) (Variables|CurrentConnectionLoop|GetRandomSelectedPossibleRoomCompatibleSocketIndex) (Variables|CurrentConnectionLoop|GetOriginRoom) (Variables|CurrentConnectionLoop|GetDerivedRoomSocket))
                          (Default|AssemblePossibleRoomConnections (Variables|StatusVariables|GetLastSpawnedDerivedRoom)))
                        (:then_2
                          ;;[0.4827 0.7843 1 0.336] Adding the new connection
                          (Utilities|Array|AddUnique (Variables|StatusVariables|GetEstablishedConnections) (Utilities|Struct|MakeRoomConnection (Variables|CurrentConnectionLoop|GetOriginRoom) (Utilities|Array|Get(acopy) (Variables|/Game/Work_Hassene/Prefabs/Master/BPP_BaseRoom.BPP_BaseRoom_C|GetSockets (Variables|CurrentConnectionLoop|GetOriginRoom)) (Variables|CurrentConnectionLoop|GetOriginRoomSocketIndex)) (Variables|StatusVariables|GetLastSpawnedDerivedRoom) (Utilities|Array|Get(acopy) (Variables|/Game/Work_Hassene/Prefabs/Master/BPP_BaseRoom.BPP_BaseRoom_C|GetSockets (Variables|StatusVariables|GetLastSpawnedDerivedRoom)) (Variables|CurrentConnectionLoop|GetRandomSelectedPossibleRoomCompatibleSocketIndex)))))))
                    (:then_3)
                    (:then_4
                      (Class|BPILevelGeneration|ProcessNextOriginRoomSocket(Message) self)))))))
          (else
            ;;[1 0 0.9922 0.073] Removing origin room from queue
            (Utilities|Array|RemoveItem (Variables|StatusVariables|GetQueuedOriginRooms) (Variables|CurrentConnectionLoop|GetOriginRoom))
            (Class|BPILevelGeneration|ProcessNextOriginRoominQueue(Message) self))))
      (:Is%20Not%20Valid
        (Development|PrintString "ORIGIN ROOM INVALID!!!" true true "(R=1.000000,G=0.000000,B=0.068793,A=1.000000)" 3e+01)))
    (else
      ;;[0 1 0.1567] Finished Generating Rooms
      (Utilities|FlowControl|Sequence
        (:then_0
          (Development|PrintString "ALL ROOMS SPAWNED." true true "(R=1.000000,G=0.000000,B=0.897633,A=1.000000)" 1e+01))
        (:then_1
          (for _array_element (Variables|StatusVariables|GetSpawnedRooms)
            (bind _asbpp_base_room (Utilities|Casting|CastToBPP_BaseRoom _array_element))
            (Default|PlugUnusedSockets _asbpp_base_room)))
        (:then_2
          (Variables|StatusVariables|SetLevelBuilt true))
        (:then_3
          (Class|BPILevelGeneration|GeneratePuzzles(Message) self))))))

(event EventGeneratePuzzles
  (bind _allspawnpoints (Variables|Default|GetAllSpawnPoints))
  (Utilities|FlowControl|Delay 5.0)
  (Utilities|FlowControl|Sequence
    (:then_0
      ;[0.4745 0.8795 1] Destroying reference rooms (Level layout generation done)
      (for _array_element (Variables|SatiticReferences|GetReferenceRooms)
        (Utilities|IsValid (Variables|/Game/Work_Hassene/Prefabs/Master/BPP_BaseRoom.BPP_BaseRoom_C|GetDecorLevelInstance _array_element)
          (:Is%20Valid
            (Class|LevelStreaming|SetIsRequestingUnloadandRemoval (Variables|/Game/Work_Hassene/Prefabs/Master/BPP_BaseRoom.BPP_BaseRoom_C|GetDecorLevelInstance _array_element) true))
          (:Is%20Not%20Valid
            _))
        (Actor|DestroyActor _array_element)
        (Utilities|FlowControl|Delay 1e+01)))
    (:then_1
      ;[0 0.08041 1] Getting all the spawn points in the level
      (bind _outactors (Actor|GetAllActorsOfClass "/Game/Work_Hassene/Blueprints/SpawnPointsContainerActors/BP_SpawnPts_Base.BP_SpawnPts_Base_C"))
      (Variables|Default|SetSpawnPointActors _outactors)
      (Development|PrintString (Utilities|String|ToString(Text) (Utilities|Text|FormatText "Spawn points ACTORS found: {X}" (Utilities|Array|Length _outactors))) true true "(R=1.000000,G=0.014812,B=0.944927,A=1.000000)" 2e+01)
      (for _array_element_2 _outactors
        (for _array_element_3 (Variables|/Game/Work_Hassene/Blueprints/SpawnPointsContainerActors/BP_SpawnPts_Base.BP_SpawnPts_Base_C|GetSpawnPoints _array_element_2)
          (Utilities|Array|AddUnique (Variables|Default|GetAllSpawnPoints) _array_element_3)))
      (if (Utilities|Array|IsEmpty _allspawnpoints)
        (Development|PrintString "SPAWN POINTS EMPTY" true true "(R=1.000000,G=0.039298,B=0.000000,A=1.000000)" 2e+01)
        (else
          (Development|PrintString (Utilities|String|ToString(Text) (Utilities|Text|FormatText "Spawn points found: {X}" (Utilities|Array|Length _allspawnpoints))) true true "(R=0.000000,G=0.932967,B=1.000000,A=1.000000)" 2e+01))))
    (:then_2
      (if (Utilities|Array|IsNotEmpty (Variables|Default|GetAllSpawnPoints))
        (for _array_element_4 (Variables|Default|GetPuzzleStuffToSpawn)
          (Utilities|FlowControl|Sequence
            (:then_0
              ;[0.1756 0.1667 1] Filter by compatibility and if already used or not
              (bind _filteredarray (CallFunction|FilterSpawnPointsbyCompatibility (Variables|Default|GetAllSpawnPoints) (Utilities|Array|Get(acopy) (Variables|/Script/Engine.Actor|GetTags _array_element_4))))
              (Variables|Default|SetFilteredCompatibleSpawnPoints _filteredarray))
            (:then_1
              (if (Utilities|Array|IsNotEmpty (Variables|Default|GetFilteredCompatibleSpawnPoints))
                (Variables|Default|SetTempPickedSpawnPoint (.OutItem (Utilities|Array|Random (Variables|Default|GetFilteredCompatibleSpawnPoints))))
                (Transformation|SetActorLocation _array_element_4 (.worldlocation (Variables|Default|GetTempPickedSpawnPoint)) false false)
                (Transformation|SetActorRotation _array_element_4 (.rotation (.relativelocation (Variables|Default|GetTempPickedSpawnPoint))))
                (Class|Actor|AddActorWorldRotation _array_element_4 "0.000000,90.000000,0.000000")
                (bind _returnvalue (Utilities|Array|RemoveItem (Variables|Default|GetAllSpawnPoints) (Variables|Default|GetTempPickedSpawnPoint)))
                (Variables|Default|SetTempPickedSpawnPoint "")
                (if _returnvalue
                  (Development|PrintString (Utilities|String|ToString(Text) (Utilities|Text|FormatText "{X} was set" (Utilities|GetClassDisplayName (Utilities|GetClass _array_element_4)))) true true "(R=1.000000,G=0.000000,B=0.925167,A=1.000000)" 2e+01)
                  (else
                    (Development|PrintString "COULDNT REMOVE ITEM FROM ARRAY" true true "(R=1.000000,G=0.018152,B=0.000000,A=1.000000)" 2e+01)))
                (else
                  (Development|PrintString (Utilities|String|ToString(Text) (Utilities|Text|FormatText "DID NOT FIND ANY compatible socket, actors tag is: {x}" (Utilities|Array|Get(acopy) (Variables|/Script/Engine.Actor|GetTags _array_element_4)))) true true "(R=1.000000,G=0.040734,B=0.000000,A=1.000000)" 2e+01))))
            (:then_2
              (Utilities|Array|Clear (Variables|Default|GetFilteredCompatibleSpawnPoints)))))
        (else
          (Development|PrintString "NO SPAWN POINTS" true true "(R=1.000000,G=0.000000,B=0.125748,A=1.000000)"))))
    (:then_3
      ;[0.000229 0.005208 0.004585] Randomized Spawning for Flashlight Batteries & Taser Ammo
      (Utilities|FlowControl|Sequence
        (:then_0
          (Utilities|Array|Clear (Variables|Default|GetFilteredCompatibleSpawnPoints))
          (bind _filteredarray_2 (CallFunction|FilterSpawnPointsbyCompatibility (Variables|Default|GetAllSpawnPoints) "SmallItem"))
          (Variables|Default|SetFilteredCompatibleSpawnPoints _filteredarray_2))
        (:then_1
          (if (Utilities|Array|IsNotEmpty (Variables|Default|GetFilteredCompatibleSpawnPoints))
            (Utilities|FlowControl|Sequence
              (:then_0
                (while (< (Variables|Default|GetBatteriesSpawned) (Variables|Default|GetNumberOfBatteries))
                  (bind _output_get (Variables|Default|SetTempPickedSpawnPoint (.OutItem (Utilities|Array|Random (Variables|Default|GetFilteredCompatibleSpawnPoints)))))
                  (if (.used _output_get)
                    _
                    (else
                      (Game|SpawnActorfromClass "/Game/HorrorMechanics/Blueprint/BP_InventoryItem.BP_InventoryItem_C" (Math|Conversions|ToTransform(Vector) (.worldlocation (Variables|Default|GetTempPickedSpawnPoint))) "Undefined" "MultiplyWithRoot" 0 "/Game/HorrorMechanics/Database/InventoryItems/BP_Battery_ItemData.BP_Battery_ItemData_C" 0 -1 false false true "NewEnumerator2" "1.100000,1.100000,1.100000" false 0)
                      (Variables|Default|SetBatteriesSpawned (+ (Variables|Default|GetBatteriesSpawned) 1))
                      (Utilities|Array|SetArrayElem (Variables|Default|GetFilteredCompatibleSpawnPoints) 0 (Utilities|Struct|MakeSpawnPointData (.relativelocation (Variables|Default|GetTempPickedSpawnPoint)) (.type (Variables|Default|GetTempPickedSpawnPoint)) (.worldlocation (Variables|Default|GetTempPickedSpawnPoint)) true))))
                  (Utilities|Array|RemoveIndex (Variables|Default|GetFilteredCompatibleSpawnPoints) (.OutIndex (Utilities|Array|Random (Variables|Default|GetFilteredCompatibleSpawnPoints))))
                  (Variables|Default|SetTempPickedSpawnPoint "")
                  (Utilities|Array|RemoveItem (Variables|Default|GetAllSpawnPoints) (Variables|Default|GetTempPickedSpawnPoint))))
              (:then_1
                (while (< (Variables|Default|GetAmmoSpawned) (Variables|Default|GetNumberOfAmmo))
                  (bind _output_get_2 (Variables|Default|SetTempPickedSpawnPoint (.OutItem (Utilities|Array|Random (Variables|Default|GetFilteredCompatibleSpawnPoints)))))
                  (if (.used _output_get_2)
                    _
                    (else
                      (Game|SpawnActorfromClass "/Game/HorrorMechanics/Blueprint/BP_InventoryItem.BP_InventoryItem_C" (Math|Conversions|ToTransform(Vector) (.worldlocation (Variables|Default|GetTempPickedSpawnPoint))) "Undefined" "MultiplyWithRoot" 0 "/Game/HorrorMechanics/Database/InventoryItems/Ammo/BP_45ACP_Ammo_ItemData.BP_45ACP_Ammo_ItemData_C" 0 -1 false false true "NewEnumerator2" "1.100000,1.100000,1.100000" false 0)
                      (Variables|Default|SetAmmoSpawned (+ (Variables|Default|GetAmmoSpawned) 1))
                      (Utilities|Array|SetArrayElem (Variables|Default|GetFilteredCompatibleSpawnPoints) 0 (Utilities|Struct|MakeSpawnPointData (.relativelocation (Variables|Default|GetTempPickedSpawnPoint)) (.type (Variables|Default|GetTempPickedSpawnPoint)) (.worldlocation (Variables|Default|GetTempPickedSpawnPoint)) true))))
                  (Utilities|Array|RemoveIndex (Variables|Default|GetFilteredCompatibleSpawnPoints) (.OutIndex (Utilities|Array|Random (Variables|Default|GetFilteredCompatibleSpawnPoints))))
                  (Variables|Default|SetTempPickedSpawnPoint "")
                  (Utilities|Array|RemoveItem (Variables|Default|GetAllSpawnPoints) (Variables|Default|GetTempPickedSpawnPoint)))))
            (else
              (Development|PrintString "NO SPAWN POINTS" true true "(R=1.000000,G=0.000000,B=0.125748,A=1.000000)"))))))
    (:then_4
      ;[0.8769 1 0.4103] Door Spawning
      (Utilities|FlowControl|Sequence
        (:then_0
          ;;[1 0.6384 0.9307] Get the last spawned 5 rooms
          (bind _arrayelement (Utilities|Array|ReverseforEachLoop (Variables|StatusVariables|GetSpawnedRooms))
            (:LoopBody
              (Variables|Default|SetTempCounter (+ 1 (Variables|Default|GetTempCounter)))
              (if (>= (Variables|Default|GetTempCounter) 5)
                (Utilities|Array|AddUnique (Variables|Default|GetLast5SpawnedRooms) _arrayelement)))))
        (:then_1
          (for _array_element_5 (Variables|Default|GetDoorsToSpawn)
            (Utilities|FlowControl|Sequence
              (:then_0
                ;;[1 0.6418 0.602] Filter room sockets by connected socket
                (bind _output_get_3 (Variables|Default|SetTHE%20ROOM (Utilities|Array|Get(acopy) (Variables|Default|GetLast5SpawnedRooms) (Variables|Default|GetTempRoomIndex))))
                (bind _asbpp_base_room (Utilities|Casting|CastToBPP_BaseRoom _output_get_3))
                (for _array_element_6 (Variables|/Game/Work_Hassene/Prefabs/Master/BPP_BaseRoom.BPP_BaseRoom_C|GetSockets _asbpp_base_room)
                  (bind _output_get_4 (Variables|Default|SetTempDoorSocket _array_element_6))
                  (if (.connected (Variables|Default|GetTempDoorSocket))
                    (Utilities|Array|AddUnique (Variables|Default|GetFilteredOpenSockets) _output_get_4))))
              (:then_2
                (Utilities|FlowControl|Sequence
                  (:then_0
                    (Variables|Default|SetPicketSocketForDoor (.OutItem (Utilities|Array|Random (Variables|Default|GetFilteredOpenSockets))))
                    ;;[0.9972 1 0.6408] Convert orientation to rotator
                    (switch Utilities|FlowControl|Switch|SwitchonESocketOrientation (.orientation (Variables|Default|GetPicketSocketForDoor))
                      (:North
                        (Variables|Default|SetTempDoorRotator "0, 0, 0"))
                      (:East
                        (Variables|Default|SetTempDoorRotator "0.000000,90.000000,0.000000"))
                      (:South
                        (Variables|Default|SetTempDoorRotator "0.000000,180.000000,0.000000"))
                      (:West
                        (Variables|Default|SetTempDoorRotator "0.000000,-90.000000,0.000000"))))
                  (:then_1
                    (Game|SpawnActorfromClass (Utilities|GetClass _array_element_5) (Math|Transform|MakeTransform (+ (Transformation|GetActorLocation (Variables|Default|GetTHE%20ROOM)) (.relativelocation (Variables|Default|GetPicketSocketForDoor))) (Variables|Default|GetTempDoorRotator) "1.000000,1.000000,1.000000") "Undefined" "MultiplyWithRoot" 0 0)
                    (Variables|Default|SetTempDoorRotator "0, 0, 0")
                    (Utilities|Array|RemoveItem (Variables|Default|GetLast5SpawnedRooms) (Variables|Default|GetTHE%20ROOM))
                    (Variables|Default|SetTHE%20ROOM 0)
                    (Variables|Default|SetTempRoomIndex (+ (Variables|Default|GetTempRoomIndex) 1))
                    (Utilities|Array|Clear (Variables|Default|GetFilteredOpenSockets))
                    (Development|PrintString (Utilities|String|ToString(Text) (Utilities|Text|FormatText "{Door} spawned at a {socketOrientation} socket, rotation is {rotation}" (Utilities|GetClassDisplayName (Utilities|GetClass _array_element_5)) (Utilities|String|EnumtoString (.orientation (Variables|Default|GetPicketSocketForDoor))) (.yaw (Variables|Default|GetTempDoorRotator)))) true true "(R=0.000000,G=0.660000,B=1.000000,A=1.000000)" 6e+01)))))))))
    (:then_5
      (Utilities|FlowControl|Sequence
        (:then_0
          (Utilities|Array|Clear (Variables|Default|GetFilteredCompatibleSpawnPoints))
          (bind _filteredarray_3 (CallFunction|FilterSpawnPointsbyCompatibility (Variables|Default|GetAllSpawnPoints) "EnemySpawn"))
          (Variables|Default|SetFilteredCompatibleSpawnPoints _filteredarray_3))))))

(event EventGenerateRooms
  (bind _queuedoriginrooms (Variables|StatusVariables|GetQueuedOriginRooms))
  ;[0 0.07001 1 0.18] Level layout generation
  (if (< (Variables|StatusVariables|GetSpawnedRoomsNumber) (Variables|GenerationParameters|GetMaxRoomNumber))
    (bind _output_get (Variables|CurrentConnectionLoop|SetOriginRoom (Utilities|Array|Get(acopy) _queuedoriginrooms (Utilities|Array|LastIndex _queuedoriginrooms))))
    (Utilities|IsValid _output_get
      (:Is%20Valid
        (if (Utilities|Array|IsNotEmpty (Variables|/Game/Work_Hassene/Prefabs/Master/BPP_BaseRoom.BPP_BaseRoom_C|GetPossibleRoomConnections (Variables|CurrentConnectionLoop|GetOriginRoom)))
          (Variables|CurrentConnectionLoop|SetTempPossibleRoomConnection (Utilities|Array|Get(acopy) (Variables|/Game/Work_Hassene/Prefabs/Master/BPP_BaseRoom.BPP_BaseRoom_C|GetPossibleRoomConnections (Variables|CurrentConnectionLoop|GetOriginRoom)) (Utilities|Array|LastIndex (Variables|/Game/Work_Hassene/Prefabs/Master/BPP_BaseRoom.BPP_BaseRoom_C|GetPossibleRoomConnections (Variables|CurrentConnectionLoop|GetOriginRoom)))))
          (Utilities|FlowControl|Sequence
            (:then_0
              (Variables|CurrentConnectionLoop|SetOriginRoomSocket (.existingsocket (Variables|CurrentConnectionLoop|GetTempPossibleRoomConnection)))
              (Variables|CurrentConnectionLoop|SetOriginRoomSocketIndex (.index (Variables|CurrentConnectionLoop|GetOriginRoomSocket))))
            (:then_1
              (Variables|CurrentConnectionLoop|SetTempPossibleRoomDataArray (.possibleroomdata (Variables|CurrentConnectionLoop|GetTempPossibleRoomConnection))))
            (:then_2
              (Variables|CurrentConnectionLoop|SetRandomSelectedPossibleRoomDataIndex (.OutIndex (Utilities|Array|Random (Variables|CurrentConnectionLoop|GetTempPossibleRoomDataArray))))
              (Utilities|FlowControl|Sequence
                (:then_0
                  (Variables|CurrentConnectionLoop|SetSelectedDerivedRoom (.possibleroom (Utilities|Array|Get(acopy) (Variables|CurrentConnectionLoop|GetTempPossibleRoomDataArray) (Variables|CurrentConnectionLoop|GetRandomSelectedPossibleRoomDataIndex)))))
                (:then_1
                  (Variables|CurrentConnectionLoop|SetTempPossibleRoomsCompatibleSocketsArray (.possibleroomscompatiblesockets (Utilities|Array|Get(acopy) (Variables|CurrentConnectionLoop|GetTempPossibleRoomDataArray) (Variables|CurrentConnectionLoop|GetRandomSelectedPossibleRoomDataIndex)))))
                (:then_2
                  (Variables|CurrentConnectionLoop|SetRandomSelectedPossibleRoomCompatibleSocketIndex (.OutIndex (Utilities|Array|Random (Variables|CurrentConnectionLoop|GetTempPossibleRoomsCompatibleSocketsArray))))
                  (Variables|CurrentConnectionLoop|SetDerivedRoomSocket (Utilities|Array|Get(acopy) (Variables|CurrentConnectionLoop|GetTempPossibleRoomsCompatibleSocketsArray) (Variables|CurrentConnectionLoop|GetRandomSelectedPossibleRoomCompatibleSocketIndex)))
                  (Variables|CurrentConnectionLoop|SetRoomToConnectAnchorCoordinates (Utilities|Array|Get(acopy) (.possibleroomsanchorpoints (Utilities|Array|Get(acopy) (Variables|CurrentConnectionLoop|GetTempPossibleRoomDataArray) (Variables|CurrentConnectionLoop|GetRandomSelectedPossibleRoomDataIndex))) (Variables|CurrentConnectionLoop|GetRandomSelectedPossibleRoomCompatibleSocketIndex)))
                  (Utilities|FlowControl|Sequence
                    (:then_0
                      ;;[0.9387 0.5512 1] Spawning Room
                      (bind _returnvalue (Game|SpawnActorfromClass (Utilities|GetClass (Variables|CurrentConnectionLoop|GetSelectedDerivedRoom)) (Math|Transform|MakeTransform (Class|GridActorComponent|GetSpaceCenterWorldLocation (Variables|Default|GetGrid) (Variables|CurrentConnectionLoop|GetRoomToConnectAnchorCoordinates) (Variables|/Game/Work_Hassene/Prefabs/Master/BPP_BaseRoom.BPP_BaseRoom_C|GetSize (Variables|CurrentConnectionLoop|GetSelectedDerivedRoom))) "0, 0, 0" "1.000000,1.000000,1.000000") "AdjustIfPossibleButDontSpawnIfColliding" "MultiplyWithRoot" 0 0))
                      (bind _output_get_2 (Variables|StatusVariables|SetLastSpawnedDerivedRoom _returnvalue))
                      (Variables|/Game/Work_Hassene/Prefabs/Master/BPP_BaseRoom.BPP_BaseRoom_C|SetAnchorCoordinates _output_get_2 (Variables|CurrentConnectionLoop|GetRoomToConnectAnchorCoordinates))
                      (Default|SetupRoom (Variables|StatusVariables|GetLastSpawnedDerivedRoom)))
                    (:then_1
                      ;;[1 0.5573 0.5573] Updating grid
                      (Class|GridActorComponent|MarkSpaceOccupied (Variables|Default|GetGrid) (Variables|CurrentConnectionLoop|GetRoomToConnectAnchorCoordinates) (Variables|/Game/Work_Hassene/Prefabs/Master/BPP_BaseRoom.BPP_BaseRoom_C|GetSize (Variables|StatusVariables|GetLastSpawnedDerivedRoom)))
                      (Utilities|Array|AddUnique (Variables|StatusVariables|GetSpawnedRooms) (Variables|StatusVariables|GetLastSpawnedDerivedRoom))
                      (Math|Integer|IncrementInt (Variables|StatusVariables|GetSpawnedRoomsNumber)
                        (:%20%20
                          (Utilities|Array|AddUnique (Variables|StatusVariables|GetQueuedOriginRooms) (Variables|StatusVariables|GetLastSpawnedDerivedRoom)))))
                    (:then_2
                      ;;[0.4773 0.4503 1 0.446] Updating sockets and possible connections in each room in the established connection
                      (Utilities|FlowControl|Sequence
                        (:then_0
                          (Default|UpdateSocketsandPossibleConnections (Variables|CurrentConnectionLoop|GetOriginRoom) (Variables|CurrentConnectionLoop|GetOriginRoomSocketIndex) (Variables|StatusVariables|GetLastSpawnedDerivedRoom) (Variables|CurrentConnectionLoop|GetOriginRoomSocket))
                          (Default|AssemblePossibleRoomConnections (Variables|CurrentConnectionLoop|GetOriginRoom)))
                        (:then_1
                          (Default|UpdateSocketsandPossibleConnections (Variables|StatusVariables|GetLastSpawnedDerivedRoom) (Variables|CurrentConnectionLoop|GetRandomSelectedPossibleRoomCompatibleSocketIndex) (Variables|CurrentConnectionLoop|GetOriginRoom) (Variables|CurrentConnectionLoop|GetDerivedRoomSocket))
                          (Default|AssemblePossibleRoomConnections (Variables|StatusVariables|GetLastSpawnedDerivedRoom)))
                        (:then_2
                          ;;[0.4827 0.7843 1 0.336] Adding the new connection
                          (Utilities|Array|AddUnique (Variables|StatusVariables|GetEstablishedConnections) (Utilities|Struct|MakeRoomConnection (Variables|CurrentConnectionLoop|GetOriginRoom) (Utilities|Array|Get(acopy) (Variables|/Game/Work_Hassene/Prefabs/Master/BPP_BaseRoom.BPP_BaseRoom_C|GetSockets (Variables|CurrentConnectionLoop|GetOriginRoom)) (Variables|CurrentConnectionLoop|GetOriginRoomSocketIndex)) (Variables|StatusVariables|GetLastSpawnedDerivedRoom) (Utilities|Array|Get(acopy) (Variables|/Game/Work_Hassene/Prefabs/Master/BPP_BaseRoom.BPP_BaseRoom_C|GetSockets (Variables|StatusVariables|GetLastSpawnedDerivedRoom)) (Variables|CurrentConnectionLoop|GetRandomSelectedPossibleRoomCompatibleSocketIndex)))))))
                    (:then_3)
                    (:then_4
                      (Class|BPILevelGeneration|ProcessNextOriginRoomSocket(Message) self)))))))
          (else
            ;;[1 0 0.9922 0.073] Removing origin room from queue
            (Utilities|Array|RemoveItem (Variables|StatusVariables|GetQueuedOriginRooms) (Variables|CurrentConnectionLoop|GetOriginRoom))
            (Class|BPILevelGeneration|ProcessNextOriginRoominQueue(Message) self))))
      (:Is%20Not%20Valid
        (Development|PrintString "ORIGIN ROOM INVALID!!!" true true "(R=1.000000,G=0.000000,B=0.068793,A=1.000000)" 3e+01)))
    (else
      ;;[0 1 0.1567] Finished Generating Rooms
      (Utilities|FlowControl|Sequence
        (:then_0
          (Development|PrintString "ALL ROOMS SPAWNED." true true "(R=1.000000,G=0.000000,B=0.897633,A=1.000000)" 1e+01))
        (:then_1
          (for _array_element (Variables|StatusVariables|GetSpawnedRooms)
            (bind _asbpp_base_room (Utilities|Casting|CastToBPP_BaseRoom _array_element))
            (Default|PlugUnusedSockets _asbpp_base_room)))
        (:then_2
          (Variables|StatusVariables|SetLevelBuilt true))
        (:then_3
          (Class|BPILevelGeneration|GeneratePuzzles(Message) self))))))

(event EventProcessNextOriginRoomSocket
  (bind _originroom (Variables|CurrentConnectionLoop|GetOriginRoom))
  (bind _originroom_2 (Variables|CurrentConnectionLoop|GetOriginRoom))
  (bind _originroom_3 (Variables|CurrentConnectionLoop|GetOriginRoom))
  (bind _possibleroomconnections (Variables|/Game/Work_Hassene/Prefabs/Master/BPP_BaseRoom.BPP_BaseRoom_C|GetPossibleRoomConnections _originroom_2))
  ;[0 0.07001 1 0.18] Level layout generation
  (if (Utilities|Array|IsNotEmpty _possibleroomconnections)
    (Variables|CurrentConnectionLoop|SetTempPossibleRoomConnection (Utilities|Array|Get(acopy) _possibleroomconnections (Utilities|Array|LastIndex _possibleroomconnections)))
    (Utilities|FlowControl|Sequence
      (:then_0
        (Variables|CurrentConnectionLoop|SetOriginRoomSocket (.existingsocket (Variables|CurrentConnectionLoop|GetTempPossibleRoomConnection)))
        (Variables|CurrentConnectionLoop|SetOriginRoomSocketIndex (.index (Variables|CurrentConnectionLoop|GetOriginRoomSocket))))
      (:then_1
        (Variables|CurrentConnectionLoop|SetTempPossibleRoomDataArray (.possibleroomdata (Variables|CurrentConnectionLoop|GetTempPossibleRoomConnection))))
      (:then_2
        (Variables|CurrentConnectionLoop|SetRandomSelectedPossibleRoomDataIndex (.OutIndex (Utilities|Array|Random (Variables|CurrentConnectionLoop|GetTempPossibleRoomDataArray))))
        (Utilities|FlowControl|Sequence
          (:then_0
            (Variables|CurrentConnectionLoop|SetSelectedDerivedRoom (.possibleroom (Utilities|Array|Get(acopy) (Variables|CurrentConnectionLoop|GetTempPossibleRoomDataArray) (Variables|CurrentConnectionLoop|GetRandomSelectedPossibleRoomDataIndex)))))
          (:then_1
            (Variables|CurrentConnectionLoop|SetTempPossibleRoomsCompatibleSocketsArray (.possibleroomscompatiblesockets (Utilities|Array|Get(acopy) (Variables|CurrentConnectionLoop|GetTempPossibleRoomDataArray) (Variables|CurrentConnectionLoop|GetRandomSelectedPossibleRoomDataIndex)))))
          (:then_2
            (Variables|CurrentConnectionLoop|SetRandomSelectedPossibleRoomCompatibleSocketIndex (.OutIndex (Utilities|Array|Random (Variables|CurrentConnectionLoop|GetTempPossibleRoomsCompatibleSocketsArray))))
            (Variables|CurrentConnectionLoop|SetDerivedRoomSocket (Utilities|Array|Get(acopy) (Variables|CurrentConnectionLoop|GetTempPossibleRoomsCompatibleSocketsArray) (Variables|CurrentConnectionLoop|GetRandomSelectedPossibleRoomCompatibleSocketIndex)))
            (Variables|CurrentConnectionLoop|SetRoomToConnectAnchorCoordinates (Utilities|Array|Get(acopy) (.possibleroomsanchorpoints (Utilities|Array|Get(acopy) (Variables|CurrentConnectionLoop|GetTempPossibleRoomDataArray) (Variables|CurrentConnectionLoop|GetRandomSelectedPossibleRoomDataIndex))) (Variables|CurrentConnectionLoop|GetRandomSelectedPossibleRoomCompatibleSocketIndex)))
            (Utilities|FlowControl|Sequence
              (:then_0
                ;;[0.9387 0.5512 1] Spawning Room
                (bind _returnvalue (Game|SpawnActorfromClass (Utilities|GetClass (Variables|CurrentConnectionLoop|GetSelectedDerivedRoom)) (Math|Transform|MakeTransform (Class|GridActorComponent|GetSpaceCenterWorldLocation (Variables|Default|GetGrid) (Variables|CurrentConnectionLoop|GetRoomToConnectAnchorCoordinates) (Variables|/Game/Work_Hassene/Prefabs/Master/BPP_BaseRoom.BPP_BaseRoom_C|GetSize (Variables|CurrentConnectionLoop|GetSelectedDerivedRoom))) "0, 0, 0" "1.000000,1.000000,1.000000") "AdjustIfPossibleButDontSpawnIfColliding" "MultiplyWithRoot" 0 0))
                (bind _output_get (Variables|StatusVariables|SetLastSpawnedDerivedRoom _returnvalue))
                (Variables|/Game/Work_Hassene/Prefabs/Master/BPP_BaseRoom.BPP_BaseRoom_C|SetAnchorCoordinates _output_get (Variables|CurrentConnectionLoop|GetRoomToConnectAnchorCoordinates))
                (Default|SetupRoom (Variables|StatusVariables|GetLastSpawnedDerivedRoom)))
              (:then_1
                ;;[1 0.5573 0.5573] Updating grid
                (Class|GridActorComponent|MarkSpaceOccupied (Variables|Default|GetGrid) (Variables|CurrentConnectionLoop|GetRoomToConnectAnchorCoordinates) (Variables|/Game/Work_Hassene/Prefabs/Master/BPP_BaseRoom.BPP_BaseRoom_C|GetSize (Variables|StatusVariables|GetLastSpawnedDerivedRoom)))
                (Utilities|Array|AddUnique (Variables|StatusVariables|GetSpawnedRooms) (Variables|StatusVariables|GetLastSpawnedDerivedRoom))
                (Math|Integer|IncrementInt (Variables|StatusVariables|GetSpawnedRoomsNumber)
                  (:%20%20
                    (Utilities|Array|AddUnique (Variables|StatusVariables|GetQueuedOriginRooms) (Variables|StatusVariables|GetLastSpawnedDerivedRoom)))))
              (:then_2
                ;;[0.4773 0.4503 1 0.446] Updating sockets and possible connections in each room in the established connection
                (Utilities|FlowControl|Sequence
                  (:then_0
                    (Default|UpdateSocketsandPossibleConnections _originroom_3 (Variables|CurrentConnectionLoop|GetOriginRoomSocketIndex) (Variables|StatusVariables|GetLastSpawnedDerivedRoom) (Variables|CurrentConnectionLoop|GetOriginRoomSocket))
                    (Default|AssemblePossibleRoomConnections _originroom_3))
                  (:then_1
                    (Default|UpdateSocketsandPossibleConnections (Variables|StatusVariables|GetLastSpawnedDerivedRoom) (Variables|CurrentConnectionLoop|GetRandomSelectedPossibleRoomCompatibleSocketIndex) _originroom_3 (Variables|CurrentConnectionLoop|GetDerivedRoomSocket))
                    (Default|AssemblePossibleRoomConnections (Variables|StatusVariables|GetLastSpawnedDerivedRoom)))
                  (:then_2
                    ;;[0.4827 0.7843 1 0.336] Adding the new connection
                    (Utilities|Array|AddUnique (Variables|StatusVariables|GetEstablishedConnections) (Utilities|Struct|MakeRoomConnection _originroom (Utilities|Array|Get(acopy) (Variables|/Game/Work_Hassene/Prefabs/Master/BPP_BaseRoom.BPP_BaseRoom_C|GetSockets _originroom) (Variables|CurrentConnectionLoop|GetOriginRoomSocketIndex)) (Variables|StatusVariables|GetLastSpawnedDerivedRoom) (Utilities|Array|Get(acopy) (Variables|/Game/Work_Hassene/Prefabs/Master/BPP_BaseRoom.BPP_BaseRoom_C|GetSockets (Variables|StatusVariables|GetLastSpawnedDerivedRoom)) (Variables|CurrentConnectionLoop|GetRandomSelectedPossibleRoomCompatibleSocketIndex)))))))
              (:then_3)
              (:then_4
                (Class|BPILevelGeneration|ProcessNextOriginRoomSocket(Message) self)))))))
    (else
      ;;[1 0 0.9922 0.073] Removing origin room from queue
      (Utilities|Array|RemoveItem (Variables|StatusVariables|GetQueuedOriginRooms) (Variables|CurrentConnectionLoop|GetOriginRoom))
      (Class|BPILevelGeneration|ProcessNextOriginRoominQueue(Message) self))))

(fn GetRoomsfromDataTable
  (bind _roomsoftclassreferencesdatatable (Variables|Data|GetRoomSoftClassReferencesDataTable))
  (bind _outrownames (DataTable|GetDataTableRowNames _roomsoftclassreferencesdatatable))
  (for _array_element _outrownames
    (bind _returnvalue (Utilities|GetDataTableRow _roomsoftclassreferencesdatatable _array_element))))

(fn InitializeGenerator
  (Variables|Default|SetGrid (Actor|GetComponentbyClass (Components|GetOwner) "/Script/BlindPursuitProject.GridActorComponent"))
  (Utilities|FlowControl|Sequence
    (:then_0
      (CallFunction|SpawnAllReferenceRooms))
    (:then_1
      (bind _returnvalue (Game|SpawnActorfromClass "/Game/Work_Hassene/Prefabs/Inherit/BPP_StartRoom.BPP_StartRoom_C" (Math|Transform|MakeTransform (+ (Class|GridActorComponent|GetSpaceCenterWorldLocation (Variables|Default|GetGrid) (Variables|GenerationParameters|GetStartRoomAnchorCoordinates) "2.000000,2.000000,1.000000") (Math|Vector|MakeVector (Math|Conversions|ToFloat(Integer) (Variables|/Script/BlindPursuitProject.GridActorComponent|GetGridCellSize (Variables|Default|GetGrid))) (* (Variables|/Script/BlindPursuitProject.GridActorComponent|GetGridCellSize (Variables|Default|GetGrid)) 2) 0.0)) "0, 0, 0" "1.000000,1.000000,1.000000") "Undefined" "MultiplyWithRoot" 0 0))
      (Utilities|Array|Add (Variables|StatusVariables|GetSpawnedRooms) _returnvalue)
      (Utilities|Array|AddUnique (Variables|StatusVariables|GetQueuedOriginRooms) _returnvalue)
      (bind _output_get (Variables|/Game/Work_Hassene/Prefabs/Master/BPP_BaseRoom.BPP_BaseRoom_C|SetAnchorCoordinates _returnvalue (Variables|GenerationParameters|GetStartRoomAnchorCoordinates)))
      (Default|SetupRoom _returnvalue)
      (Default|AssemblePossibleRoomConnections _returnvalue)
      (Class|GridActorComponent|MarkSpaceOccupied (Variables|Default|GetGrid) _output_get (Variables|/Game/Work_Hassene/Prefabs/Master/BPP_BaseRoom.BPP_BaseRoom_C|GetSize _returnvalue))
      (bind _returnvalue_2 (Game|SpawnActorfromClass "/Game/Work_Hassene/Prefabs/BP_Elevator.BP_Elevator_C" (Math|Transform|MakeTransform (+ (+ (Class|GridActorComponent|GetSpaceCenterWorldLocation (Variables|Default|GetGrid) (Variables|GenerationParameters|GetStartRoomAnchorCoordinates) "2.000000,2.000000,1.000000") (Math|Vector|MakeVector (Math|Conversions|ToFloat(Integer) (Variables|/Script/BlindPursuitProject.GridActorComponent|GetGridCellSize (Variables|Default|GetGrid))) (* (Variables|/Script/BlindPursuitProject.GridActorComponent|GetGridCellSize (Variables|Default|GetGrid)) 2) 0.0)) "-210.000000,865.000000,3225.000000") "0.000000,-90.000000,0.000000" "1.000000,1.000000,1.000000") "Undefined" "MultiplyWithRoot" 0 0))
      (Variables|Default|SetElevator _returnvalue_2))
    (:then_2
      (Transformation|SetActorLocation (Game|Player|GetPlayerPawn 0) (+ (Class|GridActorComponent|GetSpaceCenterWorldLocation (Variables|Default|GetGrid) (Variables|GenerationParameters|GetStartRoomAnchorCoordinates) "2.000000,2.000000,1.000000") (Math|Vector|MakeVector (Math|Conversions|ToFloat(Integer) (Variables|/Script/BlindPursuitProject.GridActorComponent|GetGridCellSize (Variables|Default|GetGrid))) (* (Variables|/Script/BlindPursuitProject.GridActorComponent|GetGridCellSize (Variables|Default|GetGrid)) 2) 0.0)) false false))))

(fn LookforMatchingSocket
  (params (SocketToMatchWith :type Room%20Socket%20Data%20Structure) (SocketsToEvaluate :type Array%20of%20Room%20Socket%20Data%20Structures))
  (Utilities|Array|Clear (LocalVariables|GetMatchingSocketsArr))
  (LocalVariables|SetSocketToMatch SocketToMatchWith)
  (for (_array_element _array_index) SocketsToEvaluate
    (switch Utilities|FlowControl|Switch|SwitchonESocketOrientation (.orientation (Utilities|Array|Get(acopy) SocketsToEvaluate _array_index))
      (:North
        (if (Utilities|Enum|Equal(Enum) (.orientation (LocalVariables|GetSocketToMatch)) "South")
          (LocalVariables|SetSuccess true :!label _label)
          (Utilities|Array|AddUnique (LocalVariables|GetMatchingSocketsArr) _array_element)))
      (:East
        (if (Utilities|Enum|Equal(Enum) (.orientation (LocalVariables|GetSocketToMatch)) "West")
          (goto _label)))
      (:South
        (if (Utilities|Enum|Equal(Enum) (.orientation (LocalVariables|GetSocketToMatch)) "North")
          (goto _label)))
      (:West
        (if (Utilities|Enum|Equal(Enum) (.orientation (LocalVariables|GetSocketToMatch)) "East")
          (goto _label)))))
  (if (LocalVariables|GetSuccess)
    (return true (LocalVariables|GetMatchingSocketsArr))
    (else
      (return false 0))))

(fn SpawnAllReferenceRooms
  (LocalVariables|SetLastTransform (Math|Transform|MakeTransform "-10000.000000,-10000.000000,-10000.000000"))
  (for _array_element (Variables|Data|GetRoomsClassReferences)
    (bind _returnvalue (Game|SpawnActorfromClass _array_element (LocalVariables|GetLastTransform) "AlwaysSpawn" "MultiplyWithRoot" 0 0))
    (Default|SetupRoom _returnvalue)
    (Utilities|Array|AddUnique (Variables|SatiticReferences|GetReferenceRooms) _returnvalue)
    (LocalVariables|SetLastTransform (Math|Transform|MakeTransform (Math|Vector|MakeVector (+ (.x (.location (LocalVariables|GetLastTransform))) 5e+03) (.y (.location (LocalVariables|GetLastTransform))) (.z (.location (LocalVariables|GetLastTransform)))))))
  (for _array_element_2 (Variables|SatiticReferences|GetReferenceRooms)
    _)
  (return))

(fn FilterSpawnPointsbyCompatibility
  (params (Unfiltered :type Array%20of%20Spawn%20Point%20Data%20Structures) (Item%20Tag :type Name))
  (for _array_element Unfiltered
    (bind _output_get (Variables|Default|SetTestedSpawnPoint _array_element))
    (if (== Item%20Tag (Utilities|String|EnumtoString (.type (Variables|Default|GetTestedSpawnPoint))))
      (if (not (.Used (Utilities|Struct|BreakSpawnPointData _output_get)))
        (Utilities|Array|AddUnique (Variables|Default|GetFilteredArr) _output_get))))
  (return (Variables|Default|GetFilteredArr)))