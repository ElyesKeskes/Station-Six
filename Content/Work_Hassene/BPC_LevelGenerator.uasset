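; Room-based level generator component, at an early stage: it sets up data but places or connects no rooms yet.
; GetRoomsFromDataTable fills a room pool from RoomDataTable's room references.
; InitializeGenerator builds a 3D grid from GridSize and records StartRoom as the first spawned room.
; BeginPlay is empty; calls to initialization and socket-alignment rotation, plus a loop over start-room sockets, are left unwired.
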(event EventBeginPlay)

(event EventTick
  (params (DeltaSeconds :type Float%20%28single-precision%29)))

(fn GetRoomsfromDataTable
  (bind _outrownames (DataTable|GetDataTableRowNames (Variables|Default|GetRoomDataTable)))
  (for _array_element _outrownames
    (bind _returnvalue (Utilities|GetDataTableRow (Variables|Default|GetRoomDataTable) _array_element)
      (:then
        (Utilities|Array|Add (Variables|Default|GetRooms) (Utilities|Struct|BreakRoomReferenceContainer _returnvalue))))))

(fn InitializeGenerator
  (bind _gridsize (Variables|Default|GetGridSize))
  (Utilities|FlowControl|Sequence
    (:then_0
      (bind _grid (Class|LevelGenerationFLibrary|InitializeGrid (Math|Float|Truncate (.x _gridsize)) (Math|Float|Truncate (.y _gridsize)) (Math|Float|Truncate (.z _gridsize))))
      (Variables|Default|SetGrid _grid))
    (:then_1
      (Utilities|Array|Add (Variables|Default|GetSpawnedRooms) (Variables|Default|GetStartRoom)))))