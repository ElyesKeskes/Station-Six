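; Base spawn point container actor that builds its SpawnPoints list when play begins.
; Billboard components act as markers: AssembleSpawnPoints gathers them and uses each sprite texture to pick one of five spawn type enum values.
; Each entry stores relative transform, type, world location and a false flag, added uniquely.
; An unrecognized sprite leaves the temporary entry unchanged, so that value is submitted again.
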(event EventBeginPlay
  (CallFunction|AssembleSpawnPoints))

(event Collision|EventActorBeginOverlap
  (params (OtherActor :type Actor%20Object%20Reference)))

(event EventTick
  (params (DeltaSeconds :type Float%20%28single-precision%29)))

(fn ConstructionScript)

(fn AssembleSpawnPoints
  (Variables|Default|SetBillboards (Actor|GetComponentsByClass "/Script/Engine.BillboardComponent"))
  (for _array_element (Variables|Default|GetBillboards)
    (Utilities|FlowControl|Sequence
      (:then_0
        (if (== (Variables|/Script/Engine.BillboardComponent|GetSprite _array_element) "/Engine/EditorResources/Ai_Spawnpoint.Ai_Spawnpoint")
          (LocalVariables|SetTempSpawnPoint (Utilities|Struct|MakeSpawnPointData (Transformation|GetRelativeTransform _array_element) "NewEnumerator0" (Transformation|GetWorldLocation _array_element) false))
          (elif (== (Variables|/Script/Engine.BillboardComponent|GetSprite _array_element) "/Engine/EditorResources/AI/S_NavLink.S_NavLink")
            (LocalVariables|SetTempSpawnPoint (Utilities|Struct|MakeSpawnPointData (Transformation|GetRelativeTransform _array_element) "NewEnumerator2" (Transformation|GetWorldLocation _array_element) false))
            (elif (== (Variables|/Script/Engine.BillboardComponent|GetSprite _array_element) "/Engine/EditorResources/Spawn_Point.Spawn_Point")
              (LocalVariables|SetTempSpawnPoint (Utilities|Struct|MakeSpawnPointData (Transformation|GetRelativeTransform _array_element) "NewEnumerator1" (Transformation|GetWorldLocation _array_element) false))
              (elif (== (Variables|/Script/Engine.BillboardComponent|GetSprite _array_element) "/Engine/EditorMaterials/TargetIconSpawn.TargetIconSpawn")
                (LocalVariables|SetTempSpawnPoint (Utilities|Struct|MakeSpawnPointData (Transformation|GetRelativeTransform _array_element) "NewEnumerator3" (Transformation|GetWorldLocation _array_element) false))
                (elif (== (Variables|/Script/Engine.BillboardComponent|GetSprite _array_element) "/Engine/EngineDebugMaterials/TargetIcon.TargetIcon")
                  (LocalVariables|SetTempSpawnPoint (Utilities|Struct|MakeSpawnPointData (Transformation|GetRelativeTransform _array_element) "NewEnumerator4" (Transformation|GetWorldLocation _array_element) false))))))))
      (:then_1
        (Utilities|Array|AddUnique (Variables|Default|GetSpawnPoints) (LocalVariables|GetTempSpawnPoint))))))