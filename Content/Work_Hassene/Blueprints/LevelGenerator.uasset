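; LevelGenerator is an actor that sets up a grid-based level generator when play begins.
; It initializes a flat Grid, initializes the BPCLevelGenerator component, moves itself to the grid's anchor position, then triggers room generation after a short delay.
; Tick can draw the debug grid when enabled.
; An elevator descent call is present but not connected to any event.
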(event EventBeginPlay
  (bind _bpc_levelgenerator (Variables|Default|GetBPC_LevelGenerator))
  (Utilities|FlowControl|Sequence
    (:then_0
      (Class|GridActorComponent|InitializeGrid (Variables|Default|GetGrid) 20 20 1 500 "0, 0, 0"))
    (:then_1
      (Default|InitializeGenerator _bpc_levelgenerator)
      (Transformation|SetActorLocation (Variables|/Script/BlindPursuitProject.GridActorComponent|GetGridAnchorWorldPosition (Variables|Default|GetGrid)) false false)
      (Development|PrintString "LevelGenerator Actor Initialized" true true "(R=0.000000,G=1.000000,B=0.006852,A=1.000000)" 1e+01))
    (:then_2
      (Utilities|FlowControl|Delay 3.0)
      (Class|BPILevelGeneration|GenerateRooms(Message) _bpc_levelgenerator))))

(event EventTick
  (params (DeltaSeconds :type Float%20%28single-precision%29))
  (if (Variables|Default|GetDrawDebugGrid)
    (Class|GridActorComponent|DrawDebugGrid (Variables|Default|GetGrid))))

(fn ConstructionScript)