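; Elevator actor that travels to a configurable StopLocation and swings its two doors open on arrival.
; The construction script builds a relative two-point InterpToMovement path, which the StartDescent dispatcher restarts.
; When movement first stops, a short delay precedes the OpenDoors dispatcher, whose bound event plays a timeline driving both doors' yaw.
; A DoorsOpened flag, set after the delay, guards against reopening on later stops.
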(event Custom|OpenDoors_Event
  (bind _newtrack_0 (Timeline|Timeline PlayFromStart)
    (:Update
      (Utilities|FlowControl|Sequence
        (:then_0
          (Transformation|SetRelativeRotation (Variables|Default|GetRightDoor) (Math|Rotator|MakeRotator 0.0 0.0 _newtrack_0) false false))
        (:then_1
          (bind _result (Math|Float|NegateFloat _newtrack_0)
            (:%20%20
              (Transformation|SetRelativeRotation (Variables|Default|GetLeftDoor) (Math|Rotator|MakeRotator 0.0 0.0 _result) false false))))))))

(event Custom|StartDescent_Event
  (Class|InterptoMovementComponent|RestartMovement (Variables|Default|GetInterpToMovement) 1.0))

(event Custom|MovementStopped
  (params (ImpactResult :type Hit%20Result%20Structure%20%28by%20ref%29) (Time :type Float%20%28single-precision%29))
  (if (not (Variables|Default|GetDoorsOpened))
    (Utilities|FlowControl|Delay 3.0)
    (Default|CallOpenDoors)
    (Variables|Default|SetDoorsOpened true)))

(event EventBeginPlay
  (EventDispatchers|BindEventtoOpenDoors (delegate Custom|OpenDoors_Event))
  (EventDispatchers|BindEventtoStartDescent (delegate Custom|StartDescent_Event))
  (EventDispatchers|BindEventtoOnInterptoStop (Variables|Default|GetInterpToMovement) (delegate Custom|MovementStopped)))

(fn ConstructionScript
  (bind _interptomovement (Variables|Default|GetInterpToMovement))
  (Class|InterptoMovementComponent|AddControlPointPosition _interptomovement "0, 0, 0" true)
  (Class|InterptoMovementComponent|AddControlPointPosition _interptomovement (Variables|Default|GetStopLocation) true))